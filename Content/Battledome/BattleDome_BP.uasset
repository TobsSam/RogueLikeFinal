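; Battle royale-style dome actor that shrinks the play zone over time.
; After a start delay it plays a 2D sound, then runs a timeline with play rate derived from DomeDecayTime.
; The timeline scales the actor from its starting radius until ZoneCleared is set, printing the radius for debug.
; Dome overlaps trigger enter and leave zone messages on Player-tagged actors.
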(event `self.ReceiveBeginPlay`
  (bind _returnvalue_x (`KismetMathLibrary.BreakVector` (`SceneComponent.K2_GetComponentScale` (`self.battledome`))))
  (set `self.DomeRadius` _returnvalue_x)
  (bind _outactors (`GameplayStatics.GetAllActorsOfClass` "/Game/FirstPersonBP/Blueprints/FirstPersonCharacter.FirstPersonCharacter_C"))
  (set `self.Players` _outactors)
  (`KismetSystemLibrary.Delay` (`self.StartDelayTime`))
  (`GameplayStatics.SpawnSound2D` null 1.0 1.0 0.0 null)
  (`self.ZoneShrink`))

(event `ZoneShrink`
  (`TimelineComponent.SetPlayRate` (`self.ZoneShrinkTimer`) (/ 60.0 (`self.DomeDecayTime`)))
  (bind (_direction _zonepercentage) (`Timeline|ZoneShrinkTimer`)
    (:`Update`
      (if (not (`self.zoneCleared`))
        (bind _returnvalue (* _zonepercentage (`self.DomeRadius`)))
        (bind _output_get (set `self.CurrentDomeRadius` _returnvalue))
        (`KismetSystemLibrary.PrintString` (`KismetStringLibrary.Concat_StrStr` "Dome radius:" (`KismetStringLibrary.Conv_DoubleToString` _output_get)) true true (struct :`G` 0.66 :`B` 1.0 :`A` 1.0) 0.001)
        (`self.SetActorScale3D` (`KismetMathLibrary.Conv_DoubleToVector` _returnvalue))))))

(event `self.battledome.OnComponentBeginOverlap`
  (params (OverlappedComponent :type "PrimitiveComponent Object Reference") (OtherActor :type "Actor Object Reference") (OtherComp :type "PrimitiveComponent Object Reference") (OtherBodyIndex :type Integer) (bFromSweep :type Boolean) (SweepResult :type "HitResult Structure (by ref)"))
  (if (`self.ActorHasTag` OtherActor "Player")
    (message `/Game/FirstPersonBP/Blueprints/CharacterInterface.EnterZone` OtherActor)))

(event `self.battledome.OnComponentEndOverlap`
  (params (OverlappedComponent :type "PrimitiveComponent Object Reference") (OtherActor :type "Actor Object Reference") (OtherComp :type "PrimitiveComponent Object Reference") (OtherBodyIndex :type Integer))
  (if (`self.ActorHasTag` OtherActor "Player")
    (message `/Game/FirstPersonBP/Blueprints/CharacterInterface.LeaveZone` OtherActor)))

(fn `UserConstructionScript`)