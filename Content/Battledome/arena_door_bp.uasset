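; Battledome arena door that opens once all AI spawn handlers in the level are destroyed.
; One second after BeginPlay it counts the spawners, and each spawnerDestroyed event decrements that count.
; At zero, OpenDoors plays a sound and snaps two rotators to opposite pitch angles.
; It then flags every BattleDome_BP as cleared and stops its zone shrink timer.
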(event `self.ReceiveBeginPlay`
  (`KismetSystemLibrary.Delay` 1.0)
  (bind _outactors (`GameplayStatics.GetAllActorsOfClass` "/Game/AI/AISpawner/AISpawnHandler.AISpawnHandler_C"))
  (bind _output_get (set `self.Spawners` _outactors))
  (set `self.spawnerCount` (`KismetArrayLibrary.Array_Length` _output_get)))

(event `spawnerDestroyed`
  (params (Spawner :type "/Game/AI/AISpawner/AISpawnHandler Object Reference"))
  (bind _output_get (set `self.spawnerCount` (- (`self.spawnerCount`) 1)))
  (if (== _output_get 0)
    (`self.OpenDoors`)))

(event `OpenDoors`
  (`GameplayStatics.PlaySound2D` null 1.0 1.0 0.0 null null)
  (`SceneComponent.K2_SetRelativeRotation` (`self.door_1_rotator`) (`KismetMathLibrary.MakeRotator` 0.0 (* (`self.door_open_rotation`) -1.0)) false false)
  (`SceneComponent.K2_SetRelativeRotation` (`self.door_2_rotator`) (`KismetMathLibrary.MakeRotator` 0.0 (`self.door_open_rotation`)) false false)
  (bind _outactors (`GameplayStatics.GetAllActorsOfClass` "/Game/Battledome/BattleDome_BP.BattleDome_BP_C"))
  (for _array_element _outactors
    (set `/Game/Battledome/BattleDome_BP.zoneCleared` true _array_element)
    (`TimelineComponent.Stop` (`/Game/Battledome/BattleDome_BP.ZoneShrinkTimer` _array_element))))

(fn `UserConstructionScript`)